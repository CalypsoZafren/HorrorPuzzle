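; Bed is an interactable level object that serves as an objective step, unlocking the next stage for the first-person player.
; Overlap sets the character's current interact item to its InteractComponent and shows a prompt widget, and leaving clears both.
; Activation of that component sets the character's next-stage flag, changes HUD objective text to "Bed is Broken", marks itself complete and hides the prompt.
; The prompt's show condition is hardwired true, so completion does not suppress it on later overlaps.
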(event `self.ReceiveBeginPlay`
  (bind _asbp_first_person_character (cast `/Game/Blueprints/BP_FirstPersonCharacter` (`GameplayStatics.GetPlayerCharacter` 0)))
  (set `self.Character` _asbp_first_person_character))

(event `self.ReceiveActorBeginOverlap`
  (params (OtherActor :type "Actor Object Reference"))
  (bind _character (`self.Character`))
  (if (== OtherActor _character)
    (set `/Game/Blueprints/BP_FirstPersonCharacter.currentInteractItem` (`self.InteractComponent`) _character)
    (if true
      (`SceneComponent.SetHiddenInGame` (`self.InteractWidget`) false false))))

(event `self.ReceiveActorEndOverlap`
  (params (OtherActor :type "Actor Object Reference"))
  (bind _character (`self.Character`))
  (if (== OtherActor _character)
    (set `/Game/Blueprints/BP_FirstPersonCharacter.currentInteractItem` null _character)
    (`SceneComponent.SetHiddenInGame` (`self.InteractWidget`) true false)))

(event `self.InteractComponent.OnComponentActivated`
  (params (Component :type "ActorComponent Object Reference") (bReset :type Boolean))
  (bind _character (`self.Character`))
  (set `/Game/Blueprints/BP_FirstPersonCharacter.nextStageUnlocked` true _character)
  (`TextBlock.SetText` (`/Game/UI/HUD.ObjectiveText` (`/Game/Blueprints/BP_FirstPersonCharacter.HUD` _character)) "Bed is Broken")
  (set `self.isComplete` true)
  (`SceneComponent.SetHiddenInGame` (`self.InteractWidget`) true false))

(fn `UserConstructionScript`)