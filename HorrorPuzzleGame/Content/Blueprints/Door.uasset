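; Interactable door that shows a prompt and message text, and swings open with a creak when its DoorOpen event fires.
; Overlap registers its InteractComponent as the first-person character's current interact item and toggles the prompt widget, resetting its text on exit.
; Activating the component displays DoorText while the door is closed and, if RadioDoor is set, starts the linked radio's music.
; Opening is not triggered within this graph, and it disables further prompt toggling.
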(event `self.ReceiveBeginPlay`
  (bind _asbp_first_person_character (cast `/Game/Blueprints/BP_FirstPersonCharacter` (`GameplayStatics.GetPlayerCharacter` 0)))
  (set `self.Character` _asbp_first_person_character))

(event `self.ReceiveActorBeginOverlap`
  (params (OtherActor :type "Actor Object Reference"))
  (bind _character (`self.Character`))
  (if (== OtherActor _character)
    ; Sets this item as player's current iteractable item
    (set `/Game/Blueprints/BP_FirstPersonCharacter.currentInteractItem` (`self.InteractComponent`) _character)
    ; Handles UI Interaction Widget
    (if (`self.showPrompt`)
      (`SceneComponent.SetHiddenInGame` (`self.InteractWidget`) false false))))

(event `self.ReceiveActorEndOverlap`
  (params (OtherActor :type "Actor Object Reference"))
  (bind _character (`self.Character`))
  (bind _interactwidget (`self.InteractWidget`))
  (if (== OtherActor _character)
    ; Removes this item from player's current interactable item
    (set `/Game/Blueprints/BP_FirstPersonCharacter.currentInteractItem` null _character)
    ; Handles UI Interaction Widget
    (if (`self.showPrompt`)
      (`SceneComponent.SetHiddenInGame` _interactwidget true false)
      (bind _asobject_interact (cast `/Game/UI/ObjectInteract` (`WidgetComponent.GetWidget` _interactwidget)))
      (`TextBlock.SetText` (`/Game/UI/ObjectInteract.InteractText` _asobject_interact) "(Left Click) Interact"))))

(event `self.ReceiveTick`
  (params (DeltaSeconds :type "Float (single-precision)")))

(event `Door Open`
  (`SceneComponent.K2_SetRelativeRotation` (`self.Door`) (struct :`Yaw` -90.0) false false)
  (set `self.isOpen` true)
  (set `self.showPrompt` false)
  (`GameplayStatics.PlaySoundAtLocation` "/Game/Audio/DoorCreak.DoorCreak" (`self.K2_GetActorLocation`) (struct) 1.0 1.0 0.0 "/Game/Audio/NewSoundAttenuation.NewSoundAttenuation" null null null))

(event `self.InteractComponent.OnComponentActivated`
  (params (Component :type "ActorComponent Object Reference") (bReset :type Boolean))
  (`|ExecutionSequence`
    (:`then_0`
      (if (not (`self.isOpen`))
        (bind _asobject_interact (cast `/Game/UI/ObjectInteract` (`WidgetComponent.GetWidget` (`self.InteractWidget`))))
        (`TextBlock.SetText` (`/Game/UI/ObjectInteract.InteractText` _asobject_interact) (`KismetTextLibrary.Conv_StringToText` (`self.DoorText`)))))
    (:`then_1`
      (if (`self.radioDoor`)
        (`/Game/Blueprints/Radio.PlayMusic` (`self.radio`))))))

(fn `UserConstructionScript`)