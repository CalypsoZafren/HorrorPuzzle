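; BP_Book is an interactable book actor that opens a letter UI on screen for the player.
; When the first-person character overlaps it, it sets itself up as the character's current interact item and shows an interact prompt widget, clearing both on exit.
; Activation of its InteractComponent creates and adds a LetterUI widget to the viewport and hides the prompt.
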(event `self.ReceiveBeginPlay`
  (bind _asbp_first_person_character (cast `/Game/Blueprints/BP_FirstPersonCharacter` (`GameplayStatics.GetPlayerCharacter` 0)))
  (set `self.Character` _asbp_first_person_character))

(event `self.ReceiveActorBeginOverlap`
  (params (OtherActor :type "Actor Object Reference"))
  (bind _character (`self.Character`))
  (if (== OtherActor _character)
    (set `/Game/Blueprints/BP_FirstPersonCharacter.currentInteractItem` (`self.InteractComponent`) _character)
    (`SceneComponent.SetHiddenInGame` (`self.InteractWIdget`) false false)))

(event `self.ReceiveActorEndOverlap`
  (params (OtherActor :type "Actor Object Reference"))
  (bind _character (`self.Character`))
  (if (== OtherActor _character)
    (set `/Game/Blueprints/BP_FirstPersonCharacter.currentInteractItem` null _character)
    (`SceneComponent.SetHiddenInGame` (`self.InteractWIdget`) true false)))

(event `self.InteractComponent.OnComponentActivated`
  (params (Component :type "ActorComponent Object Reference") (bReset :type Boolean))
  (bind _returnvalue (`|CreateWidget` "/Game/UI/LetterUI.LetterUI_C"))
  (`UserWidget.AddToViewport` _returnvalue 0)
  (`SceneComponent.SetHiddenInGame` (`self.InteractWIdget`) true false))

(fn `UserConstructionScript`)