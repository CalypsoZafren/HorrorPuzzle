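; Interactable radio actor that advances the player's progression and arms a ghost trigger when used.
; Overlap registers its InteractComponent as the first-person character's current interact item and shows a prompt widget, clearing both on exit.
; Activating that component unlocks the next stage, hides the prompt and enables the referenced GhostTrigger.
; A separate PlayMusic event plays La Vie en Rose at the radio's location; StopMusic is an empty stub.
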(event `self.ReceiveBeginPlay`
  (bind _asbp_first_person_character (cast `/Game/Blueprints/BP_FirstPersonCharacter` (`GameplayStatics.GetPlayerCharacter` 0)))
  (set `self.Character` _asbp_first_person_character))

(event `self.ReceiveActorBeginOverlap`
  (params (OtherActor :type "Actor Object Reference"))
  (bind _character (`self.Character`))
  (if (== OtherActor _character)
    (set `/Game/Blueprints/BP_FirstPersonCharacter.currentInteractItem` (`self.InteractComponent`) _character)
    (if true
      (`SceneComponent.SetHiddenInGame` (`self.InteractWidget`) false false))))

(event `self.ReceiveActorEndOverlap`
  (params (OtherActor :type "Actor Object Reference"))
  (bind _character (`self.Character`))
  (if (== OtherActor _character)
    (set `/Game/Blueprints/BP_FirstPersonCharacter.currentInteractItem` null _character)
    (`SceneComponent.SetHiddenInGame` (`self.InteractWidget`) true false)))

(event `self.InteractComponent.OnComponentActivated`
  (params (Component :type "ActorComponent Object Reference") (bReset :type Boolean))
  (set `/Game/Blueprints/BP_FirstPersonCharacter.nextStageUnlocked` true (`self.Character`))
  (`SceneComponent.SetHiddenInGame` (`self.InteractWidget`) true false)
  (set `/Game/Blueprints/GhostMovementTrigger.shouldTrigger` true (`self.GhostTrigger`)))

(event `PlayMusic`
  (`GameplayStatics.PlaySoundAtLocation` "/Game/Audio/LA_VIE_EN_ROSE_-_EDITH_PIAF_-_M__David_-_Louiguy.LA_VIE_EN_ROSE_-_EDITH_PIAF_-_M__David_-_Louiguy" (`self.K2_GetActorLocation`) (struct) 1.0 1.0 0.0 null null null null))

(event `Stop Music`)

(fn `UserConstructionScript`)