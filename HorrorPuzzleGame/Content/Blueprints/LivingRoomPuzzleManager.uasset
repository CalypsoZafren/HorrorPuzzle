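; Manager actor for the living room puzzle that signals its completion to the player.
; On BeginPlay it casts the player pawn to BP_FirstPersonCharacter and caches it.
; Its PuzzleComplete event sets the character HUD's objective text to a completion message and flags the character's next stage as unlocked.
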(event `self.ReceiveBeginPlay`
  (bind _asbp_first_person_character (cast `/Game/Blueprints/BP_FirstPersonCharacter` (`GameplayStatics.GetPlayerPawn` 0)))
  (set `self.Character` _asbp_first_person_character))

(event `Puzzle Complete`
  (`TextBlock.SetText` (`/Game/UI/HUD.ObjectiveText` (`/Game/Blueprints/BP_FirstPersonCharacter.HUD` (`self.Character`))) (`KismetTextLibrary.Conv_StringToText` (`self.PuzzleCompleteMessage`)))
  (set `/Game/Blueprints/BP_FirstPersonCharacter.nextStageUnlocked` true (`self.Character`)))

(fn `UserConstructionScript`)