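; A one-shot trigger for a scripted ghost scare, fired when the first-person player overlaps it while ShouldTrigger is set.
; It pauses the player, and a timeline interpolates the control rotation toward Point1 while the hidden ghost is revealed there.
; A second timeline eases the ghost toward Point2, then unpauses the player, hides the ghost and destroys the trigger.
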(event `self.ReceiveBeginPlay`
  (bind _asbp_first_person_character (cast `/Game/Blueprints/BP_FirstPersonCharacter` (`GameplayStatics.GetPlayerPawn` 0)))
  (set `self.Character` _asbp_first_person_character))

(event `self.ReceiveActorBeginOverlap`
  (params (OtherActor :type "Actor Object Reference"))
  (bind _character (`self.Character`))
  (bind _ghost (`self.Ghost`))
  (bind _character_2 (`self.Character`))
  (if (and (== OtherActor _character_2) (`self.shouldTrigger`))
    (`/Game/Blueprints/BP_FirstPersonCharacter.Pause Player` _character_2)
    ; Pul lFocus to Ghost
    (`|ExecutionSequence`
      (:`then_0`
        (`/Engine/EditorBlueprintResources/StandardMacros.DoOnce` false
          (:`Completed`
            (`Timeline|CameraFocus`
              (:`Update`
                (`Controller.SetControlRotation` (`GameplayStatics.GetPlayerController` 0) (`KismetMathLibrary.RInterpTo` (`Pawn.GetControlRotation` _character) (`KismetMathLibrary.FindLookAtRotation` (`self.K2_GetActorLocation` _character) (`self.point1`)) (`GameplayStatics.GetWorldDeltaSeconds`) 2.0)))))))
      (:`then_1`
        ; Move Ghost
        (`self.SetActorHiddenInGame` _ghost false)
        (`self.K2_SetActorLocation` _ghost (`self.point1`) false false)
        (`Timeline|GhostMovement`
          (:`Update`
            (`self.K2_SetActorTransform` (`self.Ghost`) (`KismetMathLibrary.TInterpTo` (`self.GetTransform` _ghost) (`KismetMathLibrary.MakeTransform` (`self.point2`)) (`GameplayStatics.GetWorldDeltaSeconds`) 0.7) false false))
          (:`Finished`
            (`/Game/Blueprints/BP_FirstPersonCharacter.Unpause Player` (`self.Character`))
            (`self.SetActorHiddenInGame` (`self.Ghost`) true)
            (`self.K2_DestroyActor`)))))))

(fn `UserConstructionScript`)