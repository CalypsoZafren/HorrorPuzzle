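; Interactable painting in the living room puzzle that the player destroys in a fixed order once the puzzle book has been read.
; Overlap registers its InteractComponent with the first-person character and shows a prompt widget.
; Activating that component succeeds only if the preceding IndexInPuzzle item is already destroyed.
; Destruction changes the prompt text and flags LivingRoomPuzzleManager, with the third item completing the puzzle.
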(event `self.ReceiveBeginPlay`
  (`TextRenderComponent.K2_SetText` (`self.TextRender`) (`KismetTextLibrary.Conv_StringToText` (`self.paintingText`)))
  (bind _asbp_first_person_character (cast `/Game/Blueprints/BP_FirstPersonCharacter` (`GameplayStatics.GetPlayerPawn` 0)))
  (set `self.Character` _asbp_first_person_character)
  (bind _asobject_interact (cast `/Game/UI/ObjectInteract` (`WidgetComponent.GetWidget` (`self.InteractWidget`))))
  (`TextBlock.SetText` (`/Game/UI/ObjectInteract.InteractText` _asobject_interact) (`self.StartText`))
  (bind _returnvalue (`GameplayStatics.GetActorOfClass` "/Game/Blueprints/LivingRoomPuzzleManager.LivingRoomPuzzleManager_C"))
  (set `self.PuzzleManager` _returnvalue))

(event `self.ReceiveActorBeginOverlap`
  (params (OtherActor :type "Actor Object Reference"))
  (bind _character (`self.Character`))
  (if (`/Game/Blueprints/BP_Book.bookRead` (`self.PuzzleBook`))
    (if (== OtherActor _character)
      (set `/Game/Blueprints/BP_FirstPersonCharacter.currentInteractItem` (`self.InteractComponent`) _character)
      (`SceneComponent.SetHiddenInGame` (`self.InteractWIdget`) false false))))

(event `self.ReceiveActorEndOverlap`
  (params (OtherActor :type "Actor Object Reference"))
  (bind _character (`self.Character`))
  (if (== OtherActor _character)
    (set `/Game/Blueprints/BP_FirstPersonCharacter.currentInteractItem` null _character)
    (if (not (`self.destoyed`))
      (`SceneComponent.SetHiddenInGame` (`self.InteractWIdget`) true false))))

(event `self.InteractComponent.OnComponentActivated`
  (params (Component :type "ActorComponent Object Reference") (bReset :type Boolean))
  (bind _puzzlemanager (`self.PuzzleManager`))
  (if (`/Game/Blueprints/BP_Book.bookRead` (`self.PuzzleBook`))
    (switch `int` (`self.indexInPuzzle`)
      (:`1`
        (`self.Destroy Item`))
      (:`2`
        (if (`/Game/Blueprints/LivingRoomPuzzleManager.1st Item Destroyed` _puzzlemanager)
          (`self.Destroy Item`)))
      (:`3`
        (if (`/Game/Blueprints/LivingRoomPuzzleManager.2nd Item Destroyed` _puzzlemanager)
          (`self.Destroy Item`))))))

(event `Destroy Item`
  (bind _puzzlemanager (`self.PuzzleManager`))
  (bind _asobject_interact (cast `/Game/UI/ObjectInteract` (`WidgetComponent.GetWidget` (`self.InteractWidget`))))
  (set `TextBlock.Text` "Item Destroyed" (`/Game/UI/ObjectInteract.InteractText` _asobject_interact))
  (switch `int` (`self.indexInPuzzle`)
    (:`1`
      (set `/Game/Blueprints/LivingRoomPuzzleManager.1st Item Destroyed` true _puzzlemanager))
    (:`2`
      (set `/Game/Blueprints/LivingRoomPuzzleManager.2nd Item Destroyed` true _puzzlemanager))
    (:`3`
      (set `/Game/Blueprints/LivingRoomPuzzleManager.3rd Item Destroyed` true _puzzlemanager)
      (`/Game/Blueprints/LivingRoomPuzzleManager.Puzzle Complete` _puzzlemanager)))
  (set `self.destoyed` true))

(fn `UserConstructionScript`)