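; A trigger volume actor that opens a door when the player overlaps it with the next stage unlocked.
; On success it opens the linked door, shows a success message in the HUD objective text, clears the unlock flag after a short delay and destroys itself.
; Otherwise it shows an incomplete message.
; When flagged as final, it also unhides a ghost actor.
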(event `self.ReceiveBeginPlay`
  (bind _asbp_first_person_character (cast `/Game/Blueprints/BP_FirstPersonCharacter` (`GameplayStatics.GetPlayerCharacter` 0)))
  (set `self.Character` _asbp_first_person_character))

(event `self.ReceiveActorBeginOverlap`
  (params (OtherActor :type "Actor Object Reference"))
  (bind _character (`self.Character`))
  (bind _returnvalue (`KismetTextLibrary.Conv_StringToText` (`self.SuccesMessage`)))
  (bind _objectivetext (`/Game/UI/HUD.ObjectiveText` (`/Game/Blueprints/BP_FirstPersonCharacter.HUD` (`self.Character`))))
  ; Checks if Actor is Player
  (if (== OtherActor _character)
    (`|ExecutionSequence`
      (:`then_0`
        (if (`/Game/Blueprints/BP_FirstPersonCharacter.nextStageUnlocked` _character)
          (bind _objecttotrigger (`self.objectToTrigger`)
            (:`then`
              (`/Game/Blueprints/Door.Door Open` _objecttotrigger)
              (`TextBlock.SetText` _objectivetext _returnvalue)
              (`KismetSystemLibrary.Delay` 0.2)
              (set `/Game/Blueprints/BP_FirstPersonCharacter.nextStageUnlocked` false (`self.Character`))
              (`self.K2_DestroyActor`))
            (:`else`
              (`TextBlock.SetText` _objectivetext _returnvalue)))
          (else
            (`TextBlock.SetText` _objectivetext (`KismetTextLibrary.Conv_StringToText` (`self.IncompleteMessage`))))))
      (:`then_1`
        (if (`self.isFinal`)
          (`self.SetActorHiddenInGame` (`self.finalGhost`) false))))))

(fn `UserConstructionScript`)